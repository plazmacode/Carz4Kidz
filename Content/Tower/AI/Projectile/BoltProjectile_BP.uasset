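; Bolt projectile for the tower AI that knocks the off-road car on impact and expires four seconds after spawning.
; On its first hit only, the bolt turns on gravity and checks the hit actor's name against a substring before casting to OffroadCar_Pawn.
; A car hit plays a metal impact sound, applies a velocity-change impulse derived from bolt rotation to the mesh bodies, then destroys the bolt after two seconds.
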(event OnComponentHit(Bolt)
  (params (HitComponent :type Primitive%20Component%20Object%20Reference) (OtherActor :type Actor%20Object%20Reference) (OtherComp :type Primitive%20Component%20Object%20Reference) (NormalImpulse :type Vector :default "0, 0, 0") (Hit :type Hit%20Result%20Structure%20%28by%20ref%29))
  (bind _bolt (Variables|Default|GetBolt))
  (bind _returnvalue (Transformation|GetWorldTransform _bolt))
  (bind _returnvalue_2 (* (.rotation _returnvalue) 1.0))
  (Utilities|FlowControl|DoOnce false
    (:Completed
      (Physics|SetEnableGravity (Variables|Default|GetBolt) true)
      (if (Utilities|String|Contains (Utilities|GetObjectName OtherActor) (Variables|Default|GetSubstring))
        (bind _asoffroad_car_pawn (Utilities|Casting|CastToOffroadCar_Pawn OtherActor))
        (Audio|PlaySoundatLocation "/Game/Sounds/metal_impact.metal_impact" (Transformation|GetWorldLocation (Variables|Default|GetBolt)) "0, 0, 0" 1.0 1.0 0.0 0 0 0 0)
        ;[0.25 0.25 0.25] Example - Apply impulse on player
        (Class|SkeletalMeshComponent|AddImpulsetoAllBodiesBelow (Variables|/Script/ChaosVehicles.WheeledVehiclePawn|GetMesh _asoffroad_car_pawn) (Math|Vector|MakeVector (.x _returnvalue_2) (.y _returnvalue_2) (+ (.z _returnvalue_2) 0.0)) "None" true true)
        (Utilities|FlowControl|Delay 2.0)
        (Actor|DestroyActor)))))

(event EventBeginPlay
  (Utilities|FlowControl|Delay 4.0)
  (Actor|DestroyActor))

(fn ConstructionScript)