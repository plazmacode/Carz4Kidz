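; Magic attack projectile that a Magic_Pawn fires at the player's OffroadCar_Pawn, killing it on hit.
; StartProjectile grows the sphere via timeline and, after a short delay, launches it with an impulse at the pawn's LaunchSpeed.
; Aim leads the car by its velocity plus random spread, re-rolled separately for rotation and impulse.
; Any hit triggers impact sounds, particles and destruction; otherwise it self-destructs five seconds after BeginPlay.
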(event OnComponentHit(MagicSphere)
  (params (HitComponent :type Primitive%20Component%20Object%20Reference) (OtherActor :type Actor%20Object%20Reference) (OtherComp :type Primitive%20Component%20Object%20Reference) (NormalImpulse :type Vector :default "0, 0, 0") (Hit :type Hit%20Result%20Structure%20%28by%20ref%29))
  ;[0.1094 0.1094 0.1094] Component Hit
  ;;[0.25 0.25 0.25] Component is Player
  (if (Utilities|String|Contains (Utilities|GetObjectName OtherActor) (Variables|Default|GetSubstring))
    (bind _asoffroad_car_pawn (Utilities|Casting|CastToOffroadCar_Pawn OtherActor))
    (Audio|PlaySoundatLocation "/Game/Sounds/metal_impact.metal_impact" (Transformation|GetWorldLocation (Variables|Default|GetMagicSphere)) "0, 0, 0" 1.0 0.7 0.0 0 0 0 0)
    (Default|Die _asoffroad_car_pawn)
    (CallFunction|Impact)
    (else
      (CallFunction|Impact))))

(event Custom|StartProjectile
  (bind _randomness (Variables|Default|GetRandomness))
  (bind _randomness_2 (Variables|Default|GetRandomness))
  (bind _magicsphere (Variables|Default|GetMagicSphere))
  (bind _returnvalue (* _randomness -1.0))
  ;[0.1094 0.1094 0.1094] Play Magic Attack Sound
  (Variables|Default|SetSpawning true)
  (bind _returnvalue_2 (Actor|GetActorOfClass "/Game/VehicleTemplate/Blueprints/OffroadCar/OffroadCar_Pawn.OffroadCar_Pawn_C"))
  (bind _asmagic_pawn (Utilities|Casting|CastToMagic_Pawn (Variables|Default|GetMagicPawn)))
  (Audio|PlaySoundatLocation "/Game/Sounds/BigMagicAttack.BigMagicAttack" (Transformation|GetWorldLocation (Variables|/Game/Tower/AI/Magic/Magic_Pawn.Magic_Pawn_C|GetDefaultSceneRoot _asmagic_pawn)) "0, 0, 0" 0.12 1.0 0.0 0 0 0 0)
  (Utilities|FlowControl|Delay 0.7)
  ;[0.25 0.25 0.25] Set Bolt Impulse towards player
  (Transformation|SetWorldRotation _magicsphere (Math|Rotator|MakeRotator (.roll (Math|Rotator|FindLookatRotation (Transformation|GetWorldLocation (Variables|Transformation|GetRootComponent)) (+ (+ (+ (Transformation|GetWorldLocation (Variables|/Game/VehicleTemplate/Blueprints/OffroadCar/OffroadCar_Pawn.OffroadCar_Pawn_C|GetSM_Offroad_Body _returnvalue_2)) (* (Transformation|GetComponentVelocity (Variables|/Game/VehicleTemplate/Blueprints/OffroadCar/OffroadCar_Pawn.OffroadCar_Pawn_C|GetSM_Offroad_Body _returnvalue_2)) 1.0)) "") (Math|Vector|MakeVector (Math|Random|RandomFloatinRange _returnvalue _randomness_2) (Math|Random|RandomFloatinRange _returnvalue _randomness_2) (Math|Random|RandomFloatinRange _returnvalue _randomness_2))))) (.pitch (Math|Rotator|FindLookatRotation (Transformation|GetWorldLocation (Variables|Transformation|GetRootComponent)) (+ (+ (+ (Transformation|GetWorldLocation (Variables|/Game/VehicleTemplate/Blueprints/OffroadCar/OffroadCar_Pawn.OffroadCar_Pawn_C|GetSM_Offroad_Body _returnvalue_2)) (* (Transformation|GetComponentVelocity (Variables|/Game/VehicleTemplate/Blueprints/OffroadCar/OffroadCar_Pawn.OffroadCar_Pawn_C|GetSM_Offroad_Body _returnvalue_2)) 1.0)) "") (Math|Vector|MakeVector (Math|Random|RandomFloatinRange _returnvalue _randomness_2) (Math|Random|RandomFloatinRange _returnvalue _randomness_2) (Math|Random|RandomFloatinRange _returnvalue _randomness_2))))) (.yaw (Math|Rotator|FindLookatRotation (Transformation|GetWorldLocation (Variables|Transformation|GetRootComponent)) (+ (+ (+ (Transformation|GetWorldLocation (Variables|/Game/VehicleTemplate/Blueprints/OffroadCar/OffroadCar_Pawn.OffroadCar_Pawn_C|GetSM_Offroad_Body _returnvalue_2)) (* (Transformation|GetComponentVelocity (Variables|/Game/VehicleTemplate/Blueprints/OffroadCar/OffroadCar_Pawn.OffroadCar_Pawn_C|GetSM_Offroad_Body _returnvalue_2)) 1.0)) "") (Math|Vector|MakeVector (Math|Random|RandomFloatinRange _returnvalue _randomness_2) (Math|Random|RandomFloatinRange _returnvalue _randomness_2) (Math|Random|RandomFloatinRange _returnvalue _randomness_2)))))) false false)
  (Physics|AddImpulse _magicsphere (* (Math|Vector|GetForwardVector (Math|Rotator|MakeRotator (.roll (Math|Rotator|FindLookatRotation (Transformation|GetWorldLocation (Variables|Transformation|GetRootComponent)) (+ (+ (+ (Transformation|GetWorldLocation (Variables|/Game/VehicleTemplate/Blueprints/OffroadCar/OffroadCar_Pawn.OffroadCar_Pawn_C|GetSM_Offroad_Body _returnvalue_2)) (* (Transformation|GetComponentVelocity (Variables|/Game/VehicleTemplate/Blueprints/OffroadCar/OffroadCar_Pawn.OffroadCar_Pawn_C|GetSM_Offroad_Body _returnvalue_2)) 1.0)) "") (Math|Vector|MakeVector (Math|Random|RandomFloatinRange _returnvalue _randomness_2) (Math|Random|RandomFloatinRange _returnvalue _randomness_2) (Math|Random|RandomFloatinRange _returnvalue _randomness_2))))) (.pitch (Math|Rotator|FindLookatRotation (Transformation|GetWorldLocation (Variables|Transformation|GetRootComponent)) (+ (+ (+ (Transformation|GetWorldLocation (Variables|/Game/VehicleTemplate/Blueprints/OffroadCar/OffroadCar_Pawn.OffroadCar_Pawn_C|GetSM_Offroad_Body _returnvalue_2)) (* (Transformation|GetComponentVelocity (Variables|/Game/VehicleTemplate/Blueprints/OffroadCar/OffroadCar_Pawn.OffroadCar_Pawn_C|GetSM_Offroad_Body _returnvalue_2)) 1.0)) "") (Math|Vector|MakeVector (Math|Random|RandomFloatinRange _returnvalue _randomness_2) (Math|Random|RandomFloatinRange _returnvalue _randomness_2) (Math|Random|RandomFloatinRange _returnvalue _randomness_2))))) (.yaw (Math|Rotator|FindLookatRotation (Transformation|GetWorldLocation (Variables|Transformation|GetRootComponent)) (+ (+ (+ (Transformation|GetWorldLocation (Variables|/Game/VehicleTemplate/Blueprints/OffroadCar/OffroadCar_Pawn.OffroadCar_Pawn_C|GetSM_Offroad_Body _returnvalue_2)) (* (Transformation|GetComponentVelocity (Variables|/Game/VehicleTemplate/Blueprints/OffroadCar/OffroadCar_Pawn.OffroadCar_Pawn_C|GetSM_Offroad_Body _returnvalue_2)) 1.0)) "") (Math|Vector|MakeVector (Math|Random|RandomFloatinRange _returnvalue _randomness_2) (Math|Random|RandomFloatinRange _returnvalue _randomness_2) (Math|Random|RandomFloatinRange _returnvalue _randomness_2))))))) (Variables|/Game/Tower/AI/Magic/Magic_Pawn.Magic_Pawn_C|GetLaunchSpeed _asmagic_pawn)) "None" true))

(event Custom|Impact
  (bind _magicsphere (Variables|Default|GetMagicSphere))
  (bind _returnvalue (Transformation|GetWorldLocation _magicsphere))
  (bind (_x _y) (Class|KismetMathLibrary|BreakVector3f _returnvalue))
  (Audio|PlaySoundatLocation "/Game/StarterContent/Audio/Explosion01.Explosion01" _returnvalue "0, 0, 0" 0.5 0.2 0.0 0 0 0 0)
  (Audio|PlaySoundatLocation "/Game/Sounds/magicImpact.magicImpact" "0, 0, 0" "0, 0, 0" 0.4 0.8 0.0 0 0 0 0)
  (Effects|SpawnEmitteratLocation "/Game/Tower/FXVarietyPack/Particles/P_ky_ThunderBallHit.P_ky_ThunderBallHit" (Math|Vector|MakeVector _x _y 0.0) "0, 0, 0" "3.000000,3.000000,3.000000")
  (Actor|DestroyActor))

(event EventBeginPlay
  (Utilities|FlowControl|Delay 5.0)
  (Actor|DestroyActor))

(event EventTick
  (params (DeltaSeconds :type Float%20%28single-precision%29))
  ;[0.1094 0.1094 0.1094] Increase projectile size with timeline, if Spawning is true
  (if (Variables|Default|GetSpawning)
    (bind _scale_float (Timeline|Timeline Play)
      (:Update
        (Transformation|SetWorldScale3D (Variables|Default|GetMagicSphere) (Math|Vector|MakeVector _scale_float _scale_float _scale_float)))
      (:Finished
        (Variables|Default|SetSpawning false)))))

(fn ConstructionScript)